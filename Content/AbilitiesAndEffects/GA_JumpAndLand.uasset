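; Gameplay ability for a targeted leap that knocks nearby characters away on landing.
; A player-confirmed target point shapes an arced spline on the caster, whose StartJumpAndLand begins the jump.
; On the Landed gameplay event, the authority spawns an actor and distortion emitter, then launches overlapping BP_UnknownChar pawns away from the caster.
; EndAbility runs only inside that launch loop, so a landing that hits nobody never ends the ability.
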(event `self.K2_ActivateAbility`
  (bind _abilitycaster (`self.AbilityCaster`))
  (bind _jumpto (`self.JumpTo`))
  (bind _jumpdistance (`self.JumpDistance`))
  (bind (_locationtype _literaltransform _sourceactor _sourcecomponent _sourceability _sourcesocketname) (break `GameplayAbilityTargetingLocationInfo` (`self.MakeTargetLocationInfoFromOwnerActor`)))
  (bind _returnvalue (`Actor.K2_GetActorLocation` (`self.AbilityCaster`)))
  (bind _spline (`/Game/ThirdPersonCPP/Blueprints/BP_UnknownChar.Spline` (`self.AbilityCaster`)))
  (`parent.K2_ActivateAbility`)
  (bind (_asynctaskproxy _data) (`AbilityTask_WaitTargetData.WaitTargetData` "None" "UserConfirmed" "/Game/BP_TargetActor.BP_TargetActor_C" 0.0 0.0 1500.0 (struct :`Name` "NoCollision") true (make `GameplayAbilityTargetingLocationInfo` _locationtype (`KismetMathLibrary.MakeTransform` (+ (.location _literaltransform) (* (`Actor.GetActorForwardVector` (`self.AbilityCaster`)) 200.0)) (.rotation _literaltransform) (.scale _literaltransform)) _sourceactor _sourcecomponent _sourceability _sourcesocketname) (struct) null (struct) true)
    (:`ValidData`
      (bind (_bblockinghit _binitialoverlap _time _distance _location _impactpoint _normal) (`GameplayStatics.BreakHitResult` (`AbilitySystemBlueprintLibrary.GetHitResultFromTargetData` _data)))
      (bind _output_get (set `self.JumpTo` _location))
      (set `self.JumpToNormal` _normal)
      (set `self.JumpDistance` (`KismetMathLibrary.Vector_Distance` _output_get _returnvalue))
      (bind _output_get_2 (set `self.JumpFrom` _returnvalue))
      (`SplineComponent.ClearSplinePoints` _spline true)
      (`SplineComponent.SetSplinePoints` _spline (`|MakeArray` _output_get_2 (+ (* (+ (`self.JumpFrom`) _jumpto) 0.5) (`KismetMathLibrary.MakeVector` 0.0 0.0 (* _jumpdistance 0.5))) _jumpto) "World" true)
      (`SplineComponent.SetTangentAtSplinePoint` _spline 2 (* (0.0 0.0 -1.0) (`KismetMathLibrary.FClamp` _jumpdistance 0.0 2000.0)) "World" true)
      (`SceneComponent.SetVisibility` _spline true true)
      (`/Game/ThirdPersonCPP/Blueprints/BP_UnknownChar.StartJumpAndLand` (`self.AbilityCaster`))
      (`AbilityTask_WaitGameplayEvent.WaitGameplayEvent` (struct :`TagName` "Event.JumpAndLand.Landed") null
        (:`EventReceived`
          (`self.K2_HasAuthority`
            (:`True`
              (`|SpawnActorFromClass` "/Game/AdvancedMagicFX13/Blueprints/BP_ky_gaither.BP_ky_gaither_C" (`KismetMathLibrary.MakeTransform` (`self.JumpTo`) (struct) (0.5 0.5 0.5)) "AlwaysSpawn" "OverrideRootScale" _abilitycaster _abilitycaster)
              (`GameplayStatics.SpawnEmitterAtLocation` "/Game/Explosions/Particles/P_Distortion3D.P_Distortion3D")
              (bind _outactors (`KismetSystemLibrary.CapsuleOverlapActors` (`self.JumpTo`) 200.0 200.0 (`|MakeArray` "ObjectTypeQuery3" :!type "EObjectTypeQuery Enum") "/Game/ThirdPersonCPP/Blueprints/BP_UnknownChar.BP_UnknownChar_C" (`|MakeArray` (`self.AbilityCaster`) :!type "Actor Object Reference")))
              (for _array_element _outactors
                (`KismetSystemLibrary.PrintString` (`KismetSystemLibrary.GetDisplayName` _array_element))
                (bind _asbp_unknown_char (cast `/Game/ThirdPersonCPP/Blueprints/BP_UnknownChar` _array_element)
                  (:`then`
                    (`Character.LaunchCharacter` _asbp_unknown_char (* (+ (- (`Actor.K2_GetActorLocation` _array_element) (`Actor.K2_GetActorLocation` (`self.AbilityCaster`))) (* (`Actor.GetActorUpVector` _array_element) 30.0)) 10.0) true true)
                    (`self.K2_EndAbility`))
                  (:`CastFailed`
                    (`KismetSystemLibrary.PrintString` "cast failed!!!!!")))))))))
    (:`Cancelled`
      (`self.K2_CancelAbility`))))