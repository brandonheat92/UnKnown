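; Base gameplay ability for shooting a projectile, spawning a configurable projectile class from the caster's right hand.
; After committing, it plays a montage and waits once for the Event.Projectile.Shoot gameplay event to time the spawn.
; An authority check limits spawning to the server, using the caster's rotation and setting it as owner and instigator.
; The ability ends after firing or when the montage finishes or breaks off, and cancels if commit fails.
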(event `self.K2_ActivateAbility`
  (bind _abilitycaster (`self.AbilityCaster`))
  (bind _abilitycaster_2 (`self.AbilityCaster`))
  (`parent.K2_ActivateAbility`)
  (bind _returnvalue (`self.K2_CommitAbility`))
  (if _returnvalue
    (`AbilityTask_PlayMontageAndWait.CreatePlayMontageAndWaitProxy` "BaseProjectile" (`self.AnimMontToPlay`)
      (:`then`
        (`AbilityTask_WaitGameplayEvent.WaitGameplayEvent` (struct :`TagName` "Event.Projectile.Shoot") null true
          (:`EventReceived`
            (`self.HasAuthCheck`)
            (`|SpawnActorFromClass` (`self.ProjectileClass`) (`KismetMathLibrary.MakeTransform` (`SceneComponent.GetSocketLocation` (`Character.Mesh` _abilitycaster) "hand_r") (`Actor.K2_GetActorRotation` _abilitycaster)) "AlwaysSpawn" "OverrideRootScale" _abilitycaster_2 _abilitycaster_2)
            (`self.K2_EndAbility`))))
      (:`OnCompleted`
        (`self.K2_EndAbility` :!label _label))
      (:`OnBlendOut`
        (goto _label))
      (:`OnInterrupted`
        (goto _label))
      (:`OnCancelled`
        (goto _label)))
    (else
      (`self.K2_CancelAbility`))))