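; BP_ColorPickerActor is a 3D UI actor that presents a ColorPicker widget through its Widget component.
; It extends parent UI behavior for input listening, begin play, Init and Exit, keeping the widget hidden at start.
; Init triggers the picker's slide-in animation and shows it.
; Exit hides it after a fixed delay, run in a separate event because functions cannot hold a Delay.
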(event `self.ReceiveTick`
  (params (DeltaSeconds :type "Float (single-precision)")))

(event `self.ListenToUiInput`
  (params (index :type Integer))
  (`parent.ListenToUiInput` 0))

(event `self.ReceiveBeginPlay`
  (`parent.ReceiveBeginPlay`)
  (`SceneComponent.SetVisibility` (`self.Widget`) false false))

(event `DelayFromExit`
  (`KismetSystemLibrary.Delay` 1.5)
  (`SceneComponent.SetVisibility` (`self.Widget`) false false))

(fn `Exit`
  (`parent.Exit`)
  (`self.DelayFromExit`))

(fn `Init`
  (params (BlendTime :type "Float (double-precision)"))
  (`parent.Init` BlendTime)
  (bind _ascolor_picker (cast `/Game/ui/ColorPicker` (`WidgetComponent.GetUserWidgetObject` (`self.Widget`))))
  (`/Game/ui/ColorPicker.CallSlideInAnim` _ascolor_picker)
  (`SceneComponent.SetVisibility` (`self.Widget`) true false))

(fn `UserConstructionScript`)