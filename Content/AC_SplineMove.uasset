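; Actor component that places its owning character on a spline path, snapping it to the current distance along the spline every tick.
; It turns the capsule to the spline's yaw, flipped 180 degrees according to the sign of the forward input axis.
; Jumping detaches the character by clearing the path, move flag and distance.
; The component only reads the distance while moving and never advances it.
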(event `self.ReceiveTick`
  (params (DeltaSeconds :type "Float (single-precision)"))
  (`self.FollowSpline`))

(fn `FollowSpline`
  (bind (_bsuccess _asthird_person_character) (cast `` (`self.GetOwner`) :!pure true))
  (bind (_returnvalue_roll _returnvalue_pitch _returnvalue_yaw) (`KismetMathLibrary.BreakRotator` (`SplineComponent.GetRotationAtDistanceAlongSpline` (`/Game/AC_SplineMove.Spline` (`.CharacterSplinePath` (`self.CharacterSplinePath`))) (`self.DistanceAlongSpline`) "World")))
  (bind _capsulecomponent (`Character.CapsuleComponent` _asthird_person_character))
  (if (`self.Jumping`)
    (set `self.CharacterSplinePath` null)
    (set `self.MoveOnSpline` false)
    (set `self.DistanceAlongSpline` 0.0)
    (elif (`self.MoveOnSpline`)
      (`Actor.K2_SetActorLocation` _asthird_person_character (`SplineComponent.GetLocationAtDistanceAlongSpline` (`/Game/AC_SplineMove.Spline` (`.CharacterSplinePath` (`self.CharacterSplinePath`))) (`self.DistanceAlongSpline`) "World") false false)
      (set `self.CurrentRotation` (`KismetMathLibrary.MakeRotator` 0.0 0.0 _returnvalue_yaw))
      (`/Engine/EditorBlueprintResources/StandardMacros.CompareFloat` (* (`self.MoveForwardAxis`) -1.0)
        (:`>`
          (`SceneComponent.K2_SetWorldRotation` _capsulecomponent (`KismetMathLibrary.ComposeRotators` (`self.CurrentRotation`) (struct :`Yaw` 180.0)) false false))
        (:`<`
          (`SceneComponent.K2_SetWorldRotation` _capsulecomponent (`self.CurrentRotation`) false false))))))